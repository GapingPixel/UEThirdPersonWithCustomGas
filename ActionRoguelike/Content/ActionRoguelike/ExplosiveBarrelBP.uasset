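; ExplosiveBarrelBP is a networked barrel actor that explodes on its own four seconds after play begins.
; The server runs a timer that calls Explode, which triggers MulticastExplode and sets a two-second lifespan for cleanup.
; The multicast prints a debug message, fires the RadialForceComp impulse, then hides the actor and disables its collision rather than destroying it immediately.
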(event Custom|Explode
  (CallFunction|MulticastExplode)
  (Actor|SetLifeSpan 2.0))

(event Custom|MulticastExplode
  (Development|PrintString "EXPLODE!" true true "(R=0.000000,G=0.660000,B=1.000000,A=1.000000)" 1e+01)
  (Class|RadialForceComponent|FireImpulse (Variables|Default|GetRadialForceComp))
  (Rendering|SetActorHiddenInGame true)
  (Collision|SetActorEnableCollision false))

(event EventBeginPlay
  (Networking|SwitchHasAuthority
    (:Authority
      (Utilities|Time|SetTimerbyEvent (delegate Custom|Explode) 4.0))))

(event Collision|EventActorBeginOverlap
  (params (OtherActor :type Actor%20Object%20Reference)))

(event EventTick
  (params (DeltaSeconds :type Float%20%28single-precision%29)))

(fn ConstructionScript)